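; Runner manager Blueprint that spawns level parts for the runner mode and handles stopping the level.
; It caches the player runner character, then calls SpawnPart every Tick, where a Delay of GeneralSpeed divided by SpawningDelay throttles spawning of runnerPart actors at a fixed position.
; StopLevel disables Tick, zeroes the player's speed, holds the camera fully faded and shows the runner HUD widget.
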(event `self.ReceiveBeginPlay`
  (bind _as041_bp_runner_character (cast `/Game/B2/04_RunAway/041_BP_RunnerCharacter` (`GameplayStatics.GetPlayerCharacter` 0)))
  (set `self.player` _as041_bp_runner_character))

(event `SpawnPart`
  (`KismetSystemLibrary.Delay` (/ (`/Game/B2/04_RunAway/041_BP_RunnerCharacter.generalSpeed` (`self.player`)) (`self.spawningDelay`)))
  (`|SpawnActorFromClass` "/Game/B2/04_RunAway/043_runnerPart_BP.043_runnerPart_BP_C" (`KismetMathLibrary.Conv_VectorToTransform` (2050.0 0.0 0.0)) "AlwaysSpawn" "MultiplyWithRoot" null null))

(event `self.ReceiveTick`
  (params (DeltaSeconds :type "Float (single-precision)"))
  (`self.SpawnPart`))

(event `StopLevel`
  (`self.SetActorTickEnabled` false)
  (set `/Game/B2/04_RunAway/041_BP_RunnerCharacter.generalSpeed` 0.0 (`self.player`))
  (`PlayerCameraManager.StartCameraFade` :`self` (`GameplayStatics.GetPlayerCameraManager` 0) :`FromAlpha` 1.0 :`ToAlpha` 1.0 :`bHoldWhenFinished` true :!pinned true) ; From Alpha : 0\nTo Alpha : 1\nDuration : 1\nHold when Finished : TRUE
  (bind _returnvalue (`|CreateWidget` "/Game/B2/04_RunAway/DONT_TOUCH/04_runnerHUD_WB.04_runnerHUD_WB_C"))
  (`UserWidget.AddToViewport` _returnvalue 0))

(fn `UserConstructionScript`)